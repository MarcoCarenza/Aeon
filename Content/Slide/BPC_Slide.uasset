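; Character component that adds a momentum slide, started only above a speed threshold.
; StartSliding crouches, launches the character forward, cuts friction, braking and acceleration, and switches to controller-yaw rotation.
; While sliding, Tick applies gravity projected onto the floor plane to follow slopes, or small horizontal launches when airborne.
; StopSliding, called directly or by a timer, uncrouches and restores hard-coded movement settings.
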(event Custom|Start%20Sliding
  (bind _character_movement (Variables|Default|GetCharacter%20Movement))
  (bind _as_character (Variables|Default|GetAs%20Character))
  (if (> (Math|Vector|VectorLength (Variables|/Script/Engine.MovementComponent|GetVelocity (Variables|Default|GetCharacter%20Movement))) (Variables|Default|GetSlide%20Speed%20Threshold))
    (Variables|Default|SetIs%20Sliding? true)
    (Character|Crouch _as_character)
    (Character|LaunchCharacter _as_character (* (Transformation|GetActorForwardVector _as_character) (Variables|Default|GetSlide%20Impulse)) false false)
    (Variables|/Script/Engine.CharacterMovementComponent|SetGroundFriction _character_movement 0.05)
    (Variables|/Script/Engine.CharacterMovementComponent|SetBrakingDecelerationWalking _character_movement 1e+01)
    (Variables|/Script/Engine.CharacterMovementComponent|SetMaxWalkSpeedCrouched _character_movement 1.2e+03)
    (Variables|/Script/Engine.CharacterMovementComponent|SetMaxAcceleration _character_movement 0.0)
    (Variables|/Script/Engine.CharacterMovementComponent|SetbOrientRotationToMovement _character_movement false)
    (Variables|/Script/Engine.Pawn|SetbUseControllerRotationYaw (Variables|Default|GetAs%20Character) true)
    (Utilities|Time|SetTimerbyFunctionName 0 "Stop Sliding" 3.0)
    (else
      (Character|UnCrouch (Variables|Default|GetAs%20Character)))))

(event Custom|Stop%20Sliding
  (bind _character_movement (Variables|Default|GetCharacter%20Movement))
  (Variables|Default|SetIs%20Sliding? false)
  (Character|UnCrouch (Variables|Default|GetAs%20Character))
  (Variables|/Script/Engine.CharacterMovementComponent|SetGroundFriction _character_movement 8.0)
  (Variables|/Script/Engine.CharacterMovementComponent|SetBrakingDecelerationWalking _character_movement 2048.0)
  (Variables|/Script/Engine.CharacterMovementComponent|SetMaxWalkSpeedCrouched _character_movement 3e+02)
  (Variables|/Script/Engine.CharacterMovementComponent|SetMaxAcceleration _character_movement 2048.0)
  (Variables|/Script/Engine.CharacterMovementComponent|SetbOrientRotationToMovement _character_movement true)
  (Variables|/Script/Engine.Pawn|SetbUseControllerRotationYaw (Variables|Default|GetAs%20Character) false)
  (Utilities|Time|ClearTimerbyFunctionName 0 "Stop Sliding"))

(event EventBeginPlay
  (bind _ascharacter (Utilities|Casting|CastToCharacter (Components|GetOwner)))
  (bind _output_get (Variables|Default|SetAs%20Character _ascharacter))
  (Variables|Default|SetCharacter%20Movement (Variables|/Script/Engine.Character|GetCharacterMovement _output_get)))

(event EventTick
  (params (DeltaSeconds :type Float%20%28single-precision%29))
  (bind _as_character (Variables|Default|GetAs%20Character))
  (bind _returnvalue (Transformation|GetVelocity _as_character))
  (if (Variables|Default|GetIs%20Sliding?)
    (if (not (AI|Components|NavMovement|IsFalling (Variables|Default|GetCharacter%20Movement)))
      (Physics|AddForce (Variables|Default|GetCharacter%20Movement) (* (Math|Vector|ProjectVectorontoPlane (Math|Vector|MakeVector 0.0 0.0 -1.0) (.ImpactNormal (Collision|BreakHitResult (.HitResult (Utilities|Struct|BreakFindFloorResult (Variables|/Script/Engine.CharacterMovementComponent|GetCurrentFloor (Variables|Default|GetCharacter%20Movement))))))) (Variables|Default|GetSlide%20Gravity%20Force)))
      (else
        (Character|LaunchCharacter _as_character (* (Math|Vector|Normalize (Math|Vector|MakeVector (.x _returnvalue) (.y _returnvalue) 0.0)) 15.0) false false)))))